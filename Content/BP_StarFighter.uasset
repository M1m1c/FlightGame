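; BP_StarFighter is a star fighter Blueprint whose graph drives a speed-reactive camera.
; BeginPlay caches the camera's starting field of view as DefaultFOV.
; Each Tick uses MoveVelocity as a lerp alpha to lengthen the camera boom and slightly widen the FOV from that default.
; MoveVelocity is only read here, and the construction script is empty.
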(event `self.ReceiveBeginPlay`
  (set `self.DefaultFOV` (`CameraComponent.FieldOfView` (`self.CameraComp`))))

(event `self.ReceiveTick`
  (params (DeltaSeconds :type "Float (single-precision)"))
  (bind _movevelocity (`self.moveVelocity`))
  (bind _defaultfov (`self.DefaultFOV`))
  (set `SpringArmComponent.TargetArmLength` (`KismetMathLibrary.Lerp` 250.0 450.0 _movevelocity) (`self.CameraBoom`))
  (`CameraComponent.SetFieldOfView` (`self.CameraComp`) (`KismetMathLibrary.Lerp` _defaultfov (+ _defaultfov 5.0) _movevelocity)))

(fn `UserConstructionScript`)